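; Skeleton Swordman Blueprint for the dice game, handling hit and damage feedback.
; Damage taken spawns a DamageNumber widget that a timeline moves and fades, then clears before reporting done to DiceGame_GM.
; Hit events briefly set IsHit and store a HitDirection yaw derived from the forward vector and hit normal.
; The Attack event is an empty stub.
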(event Custom|Attack)

(event Custom|TakeDamage
  (params (DamagedActor :type Actor%20Object%20Reference) (Damage :type Float%20%28single-precision%29) (DamageType :type Damage%20Type%20Object%20Reference) (InstigatedBy :type Controller%20Object%20Reference) (DamageCauser :type Actor%20Object%20Reference))
  (bind _damagenumber (Variables|Default|GetDamageNumber))
  (bind _returnvalue (UserInterface|CreateWidget "/Game/SkeletonCrew/Skeleton_Swordman/DamageNumber.DamageNumber_C" 0 (Math|Float|Truncate Damage)))
  (UserInterface|SetWidget (Variables|Default|GetDamageNumber) _returnvalue)
  (bind (_direction _visibility _motion) (Timeline|DamageNumberAnimation PlayFromStart)
    (:Update
      (Utilities|FlowControl|Sequence
        (:then_0
          (Class|WidgetComponent|SetTintColorandOpacity _damagenumber (Utilities|Struct|MakeLinearColor 1.0 1.0 1.0 _visibility)))
        (:then_1
          (Transformation|SetRelativeLocation _damagenumber _motion false false))))
    (:Finished
      (UserInterface|SetWidget _damagenumber 0)
      (bind _asdice_game_gm (Utilities|Casting|CastToDiceGame_GM (Game|GetGameMode)))
      (Default|ReportDone _asdice_game_gm self))))

(event EventBeginPlay
  (EventDispatchers|BindEventtoOnTakeAnyDamage (delegate Custom|TakeDamage)))

(event Collision|EventActorBeginOverlap
  (params (OtherActor :type Actor%20Object%20Reference)))

(event EventTick
  (params (DeltaSeconds :type Float%20%28single-precision%29)))

(event Collision|EventHit
  (params (MyComp :type Primitive%20Component%20Object%20Reference) (Other :type Actor%20Object%20Reference) (OtherComp :type Primitive%20Component%20Object%20Reference) (bSelfMoved :type Boolean) (HitLocation :type Vector :default "0, 0, 0") (HitNormal :type Vector :default "0, 0, 0") (NormalImpulse :type Vector :default "0, 0, 0") (Hit :type Hit%20Result%20Structure%20%28by%20ref%29))
  (Variables|Default|SetisHit true)
  (Variables|Default|SethitDirection (.yaw (Math|Rotator|FindLookatRotation (Transformation|GetActorForwardVector) HitNormal)))
  (Utilities|FlowControl|Delay 0.2)
  (Variables|Default|SetisHit false))

(fn ConstructionScript)